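; Player character Blueprint that handles movement, mouse look and a punch attack.
; Left click plays the punch montage and enables right-hand collision, which turns off 0.5 seconds after release and at BeginPlay.
; Movement is gated by MovementEnabled: forward/back follows inverted control yaw, while left/right uses only pitch, so it ignores facing.
; Mouse look scales yaw and pitch input by frame delta time.
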(event EventBeginPlay
  (Collision|SetCollisionEnabled (Variables|Default|Getrightandcollision) "NoCollision"))

(event Collision|EventActorBeginOverlap
  (params (OtherActor :type Actor%20Object%20Reference)))

(event EventTick
  (params (DeltaSeconds :type Float%20%28single-precision%29)))

(event Input|AxisEvents|InputAxisMoveForward/Backward
  (params (AxisValue :type Float%20%28single-precision%29))
  ;[1 1 1] 플레이어 이동 (앞, 뒤)
  (if (Variables|Default|GetMovement%20Enabled)
    (Pawn|Input|AddMovementInput (Math|Vector|GetForwardVector (Math|Rotator|MakeRotator 0.0 0.0 (.yaw (Pawn|GetControlRotation :!class /Script/Engine.Pawn)))) (* AxisValue -1.0) false)))

(event Input|AxisEvents|InputAxisMoveRight/Left
  (params (AxisValue :type Float%20%28single-precision%29))
  ;[1 1 1] 플레이어 이동 (좌, 우)
  (if (Variables|Default|GetMovement%20Enabled)
    (Pawn|Input|AddMovementInput (Math|Vector|GetRightVector (Math|Rotator|MakeRotator 0.0 (.pitch (Pawn|GetControlRotation :!class /Script/Engine.Pawn)) 0.0)) (* AxisValue 1.0) false)))

(event Input|AxisEvents|InputAxisTurnRight/LeftMouse
  (params (AxisValue :type Float%20%28single-precision%29))
  ;[1 1 1] Mouse X
  (Pawn|Input|AddControllerYawInput (* AxisValue (Utilities|Time|GetWorldDeltaSeconds) 5e+01)))

(event Input|AxisEvents|InputAxisLookUp/DownMouse
  (params (AxisValue :type Float%20%28single-precision%29))
  ;[1 1 1] Mouse Y
  (Pawn|Input|AddControllerPitchInput (* AxisValue (Utilities|Time|GetWorldDeltaSeconds) 5e+01)))

(event Input|MouseEvents|RightMouseButton
  (params (Key :type Key%20Structure :default "None")))

(event Input|MouseEvents|LeftMouseButton
  (params (Key :type Key%20Structure :default "None"))
  (:Pressed
    (Animation|PlayAnimMontage "/Game/KEJ/3D_Character/Animation_Ybot/Punching1_Montage.Punching1_Montage" 1.0 "None")
    (Collision|SetCollisionEnabled (Variables|Default|Getrightandcollision) "QueryAndPhysics"))
  (:Released
    (Utilities|FlowControl|Delay 0.5)
    (Collision|SetCollisionEnabled (Variables|Default|Getrightandcollision) "NoCollision")))

(fn ConstructionScript
  (|CallParentFunction))