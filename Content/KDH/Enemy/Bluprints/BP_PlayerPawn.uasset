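; Player character Blueprint with camera-relative movement, mouse look with clamped pitch, and melee punching.
; Q punches left, E or left mouse punches right; each plays a montage and enables its hand collision until shortly after release.
; Only right-hand overlaps deal damage, calling the Enemy's Fsm OnDamageProcess and printing its HP.
; PunchL and PunchR functions play montages only; their calls in the event graph never run.
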(event OnComponentBeginOverlap(righthandcollision)
  (params (OverlappedComponent :type Primitive%20Component%20Object%20Reference) (OtherActor :type Actor%20Object%20Reference) (OtherComp :type Primitive%20Component%20Object%20Reference) (OtherBodyIndex :type Integer) (bFromSweep :type Boolean) (SweepResult :type Hit%20Result%20Structure%20%28by%20ref%29))
  (bind _asenemy (Utilities|Casting|CastToEnemy OtherActor))
  (Class|EnemyFSM|OnDamageProcess (Variables|/Script/HandToHand_MOVE.Enemy|Getfsm _asenemy))
  (Development|PrintString (Utilities|String|ToString(Integer) (Variables|/Script/HandToHand_MOVE.EnemyFSM|Gethp (Variables|/Script/HandToHand_MOVE.Enemy|Getfsm _asenemy)))))

(event EventBeginPlay
  (bind _returnvalue (Game|GetPlayerCameraManager 0))
  ;[1 1 1] 맵 각도 제한 (Pitch)
  (Variables|/Script/Engine.PlayerCameraManager|SetViewPitchMax _returnvalue 3e+01)
  (Variables|/Script/Engine.PlayerCameraManager|SetViewPitchMin _returnvalue -7e+01))

(event Collision|EventActorBeginOverlap
  (params (OtherActor :type Actor%20Object%20Reference)))

(event EventTick
  (params (DeltaSeconds :type Float%20%28single-precision%29)))

(event Input|ActionEvents|InputActionPunch_L
  (params (Key :type Key%20Structure))
  ;[1 1 1] Punch - L  :   함수 사용하여 Punch.  but, Collision 은 안됨
)

(event Input|ActionEvents|InputActionPunch_R
  (params (Key :type Key%20Structure))
  ;[1 1 1] Punch - R   :   함수 사용하여 Punch.  but, Collision 은 안됨
)

(event Input|AxisEvents|InputAxisMoveForward/Backward
  (params (AxisValue :type Float%20%28single-precision%29))
  ;[1 1 1] 플레이어 이동 (앞, 뒤)
  (if (Variables|Default|GetMovement%20Enabled)
    (Pawn|Input|AddMovementInput (Math|Vector|GetForwardVector (Math|Rotator|MakeRotator 0.0 0.0 (.yaw (Pawn|GetControlRotation :!class /Script/Engine.Pawn)))) (* AxisValue -1.0) false)))

(event Input|AxisEvents|InputAxisMoveRight/Left
  (params (AxisValue :type Float%20%28single-precision%29))
  (bind _returnvalue (Pawn|GetControlRotation :!class /Script/Engine.Pawn))
  ;[1 1 1] 플레이어 이동 (좌, 우)
  (if (Variables|Default|GetMovement%20Enabled)
    (Pawn|Input|AddMovementInput (Math|Vector|GetRightVector (Math|Rotator|MakeRotator (.roll _returnvalue) 0.0 (.yaw _returnvalue))) (* AxisValue 1.0) false)))

(event Input|AxisEvents|InputAxisTurnRight/LeftMouse
  (params (AxisValue :type Float%20%28single-precision%29))
  ;[1 1 1] Mouse X
  (Pawn|Input|AddControllerYawInput (* AxisValue (Utilities|Time|GetWorldDeltaSeconds) 5e+01)))

(event Input|AxisEvents|InputAxisLookUp/DownMouse
  (params (AxisValue :type Float%20%28single-precision%29))
  ;[1 1 1] Mouse Y
  (Pawn|Input|AddControllerPitchInput (* AxisValue (Utilities|Time|GetWorldDeltaSeconds) 5e+01)))

(event Input|KeyboardEvents|E
  (params (Key :type Key%20Structure))
  (:Pressed
    ;[1 1 1] Punch - R
    (Animation|PlayAnimMontage "/Game/KEJ/Animations/AMtg_Punch_R.AMtg_Punch_R" 1.0 "None")
    (Collision|SetCollisionEnabled (Variables|Default|Getrighthandcollision) "QueryAndPhysics"))
  (:Released
    (Utilities|FlowControl|Delay 0.5)
    (Collision|SetCollisionEnabled (Variables|Default|Getrighthandcollision) "NoCollision")))

(event Input|MouseEvents|LeftMouseButton
  (params (Key :type Key%20Structure))
  ;[1 1 1] Punch - R
  (:Pressed
    (Animation|PlayAnimMontage "/Game/KEJ/Animations/AMtg_Punch_R.AMtg_Punch_R" 1.0 "None")
    (Collision|SetCollisionEnabled (Variables|Default|Getrighthandcollision) "QueryAndPhysics"))
  (:Released
    (Utilities|FlowControl|Delay 0.5)
    (Collision|SetCollisionEnabled (Variables|Default|Getrighthandcollision) "NoCollision")))

(event Input|KeyboardEvents|Q
  (params (Key :type Key%20Structure))
  ;[1 1 1] Punch - L
  (:Pressed
    (Animation|PlayAnimMontage "/Game/KEJ/Animations/AMtg_Punch_L.AMtg_Punch_L" 1.0 "None")
    (Collision|SetCollisionEnabled (Variables|Default|Getlefthandcollision) "QueryAndPhysics"))
  (:Released
    (Utilities|FlowControl|Delay 0.5)
    (Collision|SetCollisionEnabled (Variables|Default|Getlefthandcollision) "NoCollision")))

(fn ConstructionScript
  (|CallParentFunction))

(fn PunchR
  (Animation|PlayAnimMontage "/Game/KEJ/Animations/AMtg_Punch_R.AMtg_Punch_R" 1.0 "None"))

(fn PunchL
  (Animation|PlayAnimMontage "/Game/KEJ/Animations/AMtg_Punch_L.AMtg_Punch_L" 1.0 "None"))