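; BP_Enemy_v3 is an enemy Blueprint that damages the player through contact with its fists and feet.
; Each of its four limb collision boxes handles begin overlap, casts the other actor to BP_PlayerPawn and calls ReceiveDamage with a fixed amount.
; The graph does not gate hits by attack state, and BeginPlay, Tick and the construction script are empty.
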(event OnComponentBeginOverlap(LeftFistCollisionBox)
  (params (OverlappedComponent :type Primitive%20Component%20Object%20Reference) (OtherActor :type Actor%20Object%20Reference) (OtherComp :type Primitive%20Component%20Object%20Reference) (OtherBodyIndex :type Integer) (bFromSweep :type Boolean) (SweepResult :type Hit%20Result%20Structure%20%28by%20ref%29))
  (bind _asbp_player_pawn (Utilities|Casting|CastToBP_PlayerPawn OtherActor))
  (Default|ReceiveDamage _asbp_player_pawn 1.0))

(event OnComponentBeginOverlap(RightFootCollisionBox)
  (params (OverlappedComponent :type Primitive%20Component%20Object%20Reference) (OtherActor :type Actor%20Object%20Reference) (OtherComp :type Primitive%20Component%20Object%20Reference) (OtherBodyIndex :type Integer) (bFromSweep :type Boolean) (SweepResult :type Hit%20Result%20Structure%20%28by%20ref%29))
  (bind _asbp_player_pawn (Utilities|Casting|CastToBP_PlayerPawn OtherActor))
  (Default|ReceiveDamage _asbp_player_pawn 1.0))

(event OnComponentBeginOverlap(LeftFootCollisionBox)
  (params (OverlappedComponent :type Primitive%20Component%20Object%20Reference) (OtherActor :type Actor%20Object%20Reference) (OtherComp :type Primitive%20Component%20Object%20Reference) (OtherBodyIndex :type Integer) (bFromSweep :type Boolean) (SweepResult :type Hit%20Result%20Structure%20%28by%20ref%29))
  (bind _asbp_player_pawn (Utilities|Casting|CastToBP_PlayerPawn OtherActor))
  (Default|ReceiveDamage _asbp_player_pawn 1.0))

(event OnComponentBeginOverlap(RightFistCollisionBox)
  (params (OverlappedComponent :type Primitive%20Component%20Object%20Reference) (OtherActor :type Actor%20Object%20Reference) (OtherComp :type Primitive%20Component%20Object%20Reference) (OtherBodyIndex :type Integer) (bFromSweep :type Boolean) (SweepResult :type Hit%20Result%20Structure%20%28by%20ref%29))
  (bind _asbp_player_pawn (Utilities|Casting|CastToBP_PlayerPawn OtherActor))
  (Default|ReceiveDamage _asbp_player_pawn 1.0))

(event EventBeginPlay)

(event Collision|EventActorBeginOverlap
  (params (OtherActor :type Actor%20Object%20Reference)))

(event EventTick
  (params (DeltaSeconds :type Float%20%28single-precision%29)))

(fn ConstructionScript)